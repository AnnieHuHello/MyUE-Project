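; BP_TriggerBox is a trigger volume that steps the player through a sequence of text objects while they stand inside it.
; Overlap by BP_FirstPersonCharacter activates it and shows the first TextSequence entry.
; While active, each Z press, received through input enabled on BeginPlay, shows the next entry and hides the previous, restarting the cycle after the last.
; Leaving the box deactivates it, resets the index and hides all entries.
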(event OnComponentBeginOverlap(riggerBox)
  (params (OverlappedComponent :type Primitive%20Component%20Object%20Reference) (OtherActor :type Actor%20Object%20Reference) (OtherComp :type Primitive%20Component%20Object%20Reference) (OtherBodyIndex :type Integer) (bFromSweep :type Boolean) (SweepResult :type Hit%20Result%20Structure%20%28by%20ref%29))
  (Development|PrintString "Overlap!")
  (Utilities|Casting|CastToBP_FirstPersonCharacter OtherActor)
  (Variables|Default|SetIsActive true)
  (Default|ShowText (Utilities|Array|Get(acopy) (Variables|Default|GetTextSequence)))
  (Variables|Default|SetCurrentIndex 1))

(event OnComponentEndOverlap(riggerBox)
  (params (OverlappedComponent :type Primitive%20Component%20Object%20Reference) (OtherActor :type Actor%20Object%20Reference) (OtherComp :type Primitive%20Component%20Object%20Reference) (OtherBodyIndex :type Integer))
  (Utilities|Casting|CastToBP_FirstPersonCharacter OtherActor)
  (Variables|Default|SetIsActive false)
  (Variables|Default|SetCurrentIndex 0)
  (for _array_element (Variables|Default|GetTextSequence)
    (Default|HideText _array_element)))

(event EventBeginPlay
  (Input|EnableInput (Game|GetPlayerController 0)))

(event Collision|EventActorBeginOverlap
  (params (OtherActor :type Actor%20Object%20Reference)))

(event EventTick
  (params (DeltaSeconds :type Float%20%28single-precision%29)))

(event Input|KeyboardEvents|Z
  (params (Key :type Key%20Structure :default "None"))
  (:Pressed
    (Development|PrintString "Z Pressed!")
    (if (Variables|Default|GetIsActive)
      (if (< (Variables|Default|GetCurrentIndex) (Utilities|Array|Length (Variables|Default|GetTextSequence)))
        (Development|PrintString "Showing text")
        (Default|ShowText (Utilities|Array|Get(acopy) (Variables|Default|GetTextSequence) (Variables|Default|GetCurrentIndex)))
        (if (> (Variables|Default|GetCurrentIndex) 0)
          (Default|HideText (Utilities|Array|Get(acopy) (Variables|Default|GetTextSequence) (- (Variables|Default|GetCurrentIndex) 1))))
        (Variables|Default|SetCurrentIndex (+ (Variables|Default|GetCurrentIndex) 1))
        (else
          (Default|HideText (Utilities|Array|Get(acopy) (Variables|Default|GetTextSequence) (- (Variables|Default|GetCurrentIndex) 1)))
          (Variables|Default|SetCurrentIndex 0))))))

(fn ConstructionScript)