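; BP_TextTrigger is a trigger actor that reveals narrative text in the world when the first-person player character overlaps its box.
; The TextWidget component starts hidden, and on overlap it becomes visible and its WB_WorldText widget receives the NarrativeText value.
; Tick rotates the widget to face the camera like a billboard.
; Nothing in the Blueprint hides the text again once shown.
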(event OnComponentBeginOverlap(TriggerBox)
  (params (OverlappedComponent :type Primitive%20Component%20Object%20Reference) (OtherActor :type Actor%20Object%20Reference) (OtherComp :type Primitive%20Component%20Object%20Reference) (OtherBodyIndex :type Integer) (bFromSweep :type Boolean) (SweepResult :type Hit%20Result%20Structure%20%28by%20ref%29))
  (bind _textwidget (Variables|Default|GetTextWidget))
  (Utilities|Casting|CastToBP_FirstPersonCharacter OtherActor)
  (Rendering|SetVisibility _textwidget true false)
  (bind _aswb_world_text (Utilities|Casting|CastToWB_WorldText (UserInterface|GetUserWidgetObject _textwidget)))
  (Variables|/Script/UMG.TextBlock|SetText (Variables|/Game/WB_WorldText.WB_WorldText_C|GetDisplayText _aswb_world_text) (Variables|Default|GetNarrativeText)))

(event EventBeginPlay
  (Rendering|SetVisibility (Variables|Default|GetTextWidget) false false))

(event Collision|EventActorBeginOverlap
  (params (OtherActor :type Actor%20Object%20Reference)))

(event EventTick
  (params (DeltaSeconds :type Float%20%28single-precision%29))
  (Transformation|SetWorldRotation (Variables|Default|GetTextWidget) (Math|Rotator|FindLookatRotation (Transformation|GetWorldLocation (Variables|Default|GetTextWidget)) (Transformation|GetActorLocation (Game|GetPlayerCameraManager 0))) false false))

(fn ConstructionScript)