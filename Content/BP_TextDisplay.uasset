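; BP_TextDisplay is an actor that displays narrative text in the world through a TextRender component.
; The text is hidden on BeginPlay; ShowText applies NarrativeText and makes it visible, and HideText hides it again.
; Logic to rotate the text toward the player camera exists in the event graph but is disconnected, so it never runs.
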(event EventBeginPlay
  (Rendering|SetVisibility (Variables|Default|GetTextRender) false false))

(event Collision|EventActorBeginOverlap
  (params (OtherActor :type Actor%20Object%20Reference)))

(event EventTick
  (params (DeltaSeconds :type Float%20%28single-precision%29)))

(fn ConstructionScript)

(fn ShowText
  (Rendering|Components|TextRender|SetText (Variables|Default|GetTextRender) (Variables|Default|GetNarrativeText))
  (Rendering|SetVisibility (Variables|Default|GetTextRender) true false))

(fn HideText
  (Rendering|SetVisibility (Variables|Default|GetTextRender) false false))