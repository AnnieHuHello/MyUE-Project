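; BP_TextDisplay_Simple is a world-space text display actor that reveals narrative text with a typewriter effect and can billboard toward the player camera.
; BeginPlay clears and hides its WB_WorldText_Simple widget and sets the draw size.
; ShowText starts a looping timer that writes one more character per tick into the widget, while HideText only hides it.
; The timer-stop check is unconnected, so the timer keeps looping.
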(event EventBeginPlay
  (bind _aswb_world_text_simple (Utilities|Casting|CastToWB_WorldText_Simple (UserInterface|GetUserWidgetObject (Variables|Default|GetTextWidget))))
  (Variables|/Game/New/WB_WorldText_Simple.WB_WorldText_Simple_C|SetNarrativeText _aswb_world_text_simple "")
  (Rendering|SetVisibility (Variables|Default|GetTextWidget) false false)
  (Class|WidgetComponent|SetDrawSize (Variables|Default|GetTextWidget) (Variables|Default|GetDrawSize)))

(event Collision|EventActorBeginOverlap
  (params (OtherActor :type Actor%20Object%20Reference)))

(event EventTick
  (params (DeltaSeconds :type Float%20%28single-precision%29))
  (if (Variables|Default|GetEnableBillboard)
    (Transformation|SetWorldRotation (Variables|Default|GetTextWidget) (Math|Rotator|FindLookatRotation (Transformation|GetWorldLocation (Variables|Default|GetTextWidget)) (Transformation|GetActorLocation (Game|GetPlayerCameraManager 0))) false false)))

(fn ConstructionScript)

(fn ShowText
  (Rendering|SetVisibility (Variables|Default|GetTextWidget) true false)
  (Variables|Default|SetFullText (Variables|Default|GetNarrativeText))
  (Variables|Default|SetCharIndex 0)
  (bind _returnvalue (Utilities|Time|SetTimerbyFunctionName 0 "TypewriterTick" 0.2 true))
  (Variables|Default|SetTypewriterTimer _returnvalue))

(fn HideText
  (Rendering|SetVisibility (Variables|Default|GetTextWidget) false false))

(fn TypewriterTick
  (bind _aswb_world_text_simple (Utilities|Casting|CastToWB_WorldText_Simple (UserInterface|GetUserWidgetObject (Variables|Default|GetTextWidget))))
  (Variables|/Game/New/WB_WorldText_Simple.WB_WorldText_Simple_C|SetNarrativeText _aswb_world_text_simple (Utilities|Text|ToText(String) (Utilities|String|Left (Utilities|String|ToString(Text) (Variables|Default|GetFullText)) (+ (Variables|Default|GetCharIndex) 1))))
  (Variables|Default|SetCharIndex (+ (Variables|Default|GetCharIndex) 1)))