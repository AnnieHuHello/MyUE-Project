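; Collectible photo actor that shows a configurable texture and scale, and is picked up with E while its box is overlapped.
; Pickup hides the photo, disables collision and stores the texture on BP_FirstPersonCharacter as CollectedPhoto.
; It then fades out a linked black cube through a looping timer that lowers a dynamic material's opacity.
; Player-facing billboard rotation is present but unconnected, and LinkedGaussianActor is unused.
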(event OnComponentBeginOverlap(Box)
  (params (OverlappedComponent :type Primitive%20Component%20Object%20Reference) (OtherActor :type Actor%20Object%20Reference) (OtherComp :type Primitive%20Component%20Object%20Reference) (OtherBodyIndex :type Integer) (bFromSweep :type Boolean) (SweepResult :type Hit%20Result%20Structure%20%28by%20ref%29))
  (if (not (Variables|Default|GetbIsPickedUp))
    (Variables|Default|SetbPlayerNearby false)
    (Development|PrintString "Press E to Pick Up")
    (Variables|Default|SetbPlayerNearby true)))

(event OnComponentEndOverlap(Box)
  (params (OverlappedComponent :type Primitive%20Component%20Object%20Reference) (OtherActor :type Actor%20Object%20Reference) (OtherComp :type Primitive%20Component%20Object%20Reference) (OtherBodyIndex :type Integer))
  (Variables|Default|SetbPlayerNearby false))

(event EventBeginPlay
  (Input|EnableInput self (Game|GetPlayerController 0))
  (bind _returnvalue (Rendering|Material|CreateDynamicMaterialInstance (Variables|Default|GetPhoto) 0 0 "None" :!class /Script/Engine.PrimitiveComponent))
  (Rendering|Material|SetTextureParameterValue _returnvalue "PhotoTex" (Variables|Default|GetPhotoTexture))
  (Transformation|SetRelativeScale3D (Variables|Default|GetPhoto) (Variables|Default|GetPhotoScale)))

(event Collision|EventActorBeginOverlap
  (params (OtherActor :type Actor%20Object%20Reference)))

(event EventTick
  (params (DeltaSeconds :type Float%20%28single-precision%29))
  ;[0.04688 0.01358 0.01592] Todo（photo Billiboard)
)

(event Input|KeyboardEvents|E
  (params (Key :type Key%20Structure :default "None"))
  (:Pressed
    (if (and (Variables|Default|GetbPlayerNearby) (not (Variables|Default|GetbIsPickedUp)))
      (Variables|Default|SetbIsPickedUp true)
      (Rendering|SetVisibility (Variables|Default|GetPhoto) false false)
      (Development|PrintString "Photo Picked Up")
      (Collision|SetActorEnableCollision false)
      (bind _asbp_first_person_character (Utilities|Casting|CastToBP_FirstPersonCharacter (Game|GetPlayerCharacter 0)))
      (bind _output_get (Variables|/Game/FirstPerson/Blueprints/BP_FirstPersonCharacter.BP_FirstPersonCharacter_C|SetCollectedPhoto _asbp_first_person_character (Variables|Default|GetPhotoTexture)))
      (Variables|Default|SetPhotoTexture _output_get)
      (bind _returnvalue (Rendering|Material|CreateDynamicMaterialInstance (Actor|GetComponentbyClass (Variables|Default|GetLinkedBlackCube) "/Script/Engine.StaticMeshComponent") 0 0 "None" :!class /Script/Engine.PrimitiveComponent))
      (Variables|Default|SetFadeMaterial _returnvalue)
      (bind _returnvalue_2 (Utilities|Time|SetTimerbyFunctionName 0 "FadeOutCube" 0.016 true))
      (Variables|Default|SetFadeTimer _returnvalue_2))))

(fn ConstructionScript)

(fn FadeOutCube
  (Variables|Default|SetFadeOpacity (- (Variables|Default|GetFadeOpacity) 0.0001))
  (Rendering|Material|SetScalarParameterValue (Variables|Default|GetFadeMaterial) "Opacity" (Variables|Default|GetFadeOpacity) :!class /Script/Engine.MaterialInstanceDynamic)
  (if (<= (Variables|Default|GetFadeOpacity) 0.0)
    (Utilities|Time|ClearandInvalidateTimerbyHandle (Variables|Default|GetFadeTimer))))